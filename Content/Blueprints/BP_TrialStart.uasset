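; BP_TrialStart is a time trial trigger: overlapping its box starts a timed run through all BP_TrialPoint actors in the level.
; It activates the points' particles, shows a W_HUD countdown and sets a timer from the goal time.
; A count event compares points with the total to declare a win.
; Winning, or re-entering while running, resets the points, removes the HUD and plays a success or failure sound.
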(event OnComponentBeginOverlap(Box)
  (params (OverlappedComponent :type Primitive%20Component%20Object%20Reference) (OtherActor :type Actor%20Object%20Reference) (OtherComp :type Primitive%20Component%20Object%20Reference) (OtherBodyIndex :type Integer) (bFromSweep :type Boolean) (SweepResult :type Hit%20Result%20Structure%20%28by%20ref%29))
  (bind _trial_points (Variables|Default|GetTrial%20Points))
  (Class|BPITimeTrial|TimeTrialStart(Message) OtherActor self)
  (for _array_element _trial_points
    (Components|Activation|SetActive (Variables|/Game/Blueprints/BP_TrialPoint.BP_TrialPoint_C|GetParticleSystem _array_element) true false))
  (Variables|Default|SetTrialTime (Math|Timespan|MakeTimespan 0 0 0 25))
  (if (Variables|Default|GetRunning)
    (Variables|Default|SetWin false)
    (CallFunction|ResetTimer)
    (else
      (Variables|Default|SetRunning true)
      (Variables|Default|SetTotalPoints (Utilities|Array|Length _trial_points))
      (Audio|PlaySound2D "/Engine/VREditor/Sounds/UI/Click_on_Button.Click_on_Button" 1.0 1.0 0.0 0 0)
      (CallFunction|TimeTrialHUD))))

(event Custom|EndTrial
  (params (Win :type Boolean))
  (for _array_element (Variables|Default|GetTrial%20Points)
    (Class|BPITimeTrial|TimeTrialReset(Message) _array_element))
  (if Win
    (Utilities|FlowControl|Delay 0.2)
    (Audio|PlaySound2D "/Engine/EditorSounds/Notifications/CompileSuccess.CompileSuccess" 1.0 1.0 0.0 0 0)
    (else
      (Utilities|FlowControl|Delay 0.2)
      (Audio|PlaySound2D "/Engine/EditorSounds/Notifications/CompileFailed.CompileFailed" 1.0 1.0 0.0 0 0))))

(event Custom|TimeTrialHUD
  ;[0.15 0.15 0.15 0.5] Creates widget (Change if widget is done in 3p character
  (bind _returnvalue (UserInterface|CreateWidget "/Game/Widgets/W_HUD.W_HUD_C" (Game|GetPlayerController 0)))
  (bind _output_get (Variables|Default|SetHUD _returnvalue))
  (UserInterface|Viewport|AddtoViewport _output_get 0)
  (Utilities|FlowControl|Sequence
    (:then_0
      (Widget|SetVisibility (Variables|/Game/Widgets/W_HUD.W_HUD_C|GetW_Timer (Variables|Default|GetHUD)) "Visible"))
    (:then_1
      ;[0.15 0.15 0.15 0.5] Trial time counts down
      (Default|StartTimer (Variables|/Game/Widgets/W_HUD.W_HUD_C|GetW_Timer (Variables|Default|GetHUD)) false)
      ;[0.15 0.15 0.15 0.5] Timer for tial
      (Default|SetTime (Variables|/Game/Widgets/W_HUD.W_HUD_C|GetW_Timer (Variables|Default|GetHUD)) (Variables|Default|GetTrialTime))
      ;[0.15 0.15 0.15 0.5] Goal of time trial
      (bind _time (Default|SetGoal (Variables|/Game/Widgets/W_HUD.W_HUD_C|GetW_Timer (Variables|Default|GetHUD)) 0 0 0 (Variables|Default|GetTrialTime)))
      (bind _returnvalue_2 (Utilities|Time|SetTimerbyEvent (EventDispatchers|CreateEvent :!event Custom|ResetTimer) _time))
      (Variables|Default|SetReset _returnvalue_2))))

(event Custom|ResetTimer
  (bind _hud (Variables|Default|GetHUD))
  (bind _w_timer (Variables|/Game/Widgets/W_HUD.W_HUD_C|GetW_Timer _hud))
  (Widget|SetVisibility _w_timer "Visible")
  (Variables|Default|SetRunning false)
  (Variables|Default|SetTotalPoints 0)
  (CallFunction|EndTrial (Variables|Default|GetWin))
  (Default|ClearTimer _w_timer)
  ;[0.15 0.15 0.15 0.5] Might not need this if done in 3rd person character
  (Widget|RemovefromParent (Variables|Default|GetHUD))
  (Utilities|Time|ClearandInvalidateTimerbyHandle (Variables|Default|GetReset))
  (Variables|Default|SetWin false))

(event Custom|Test
  ;[0.15 0.15 0.15 0.5] For testing purpose
  (Development|PrintString "Hello"))

(event EventBeginPlay
  (bind _outactors (Actor|GetAllActorsOfClass "/Game/Blueprints/BP_TrialPoint.BP_TrialPoint_C"))
  (Variables|Default|SetTrial%20Points _outactors))

(event EventTimeTrialCount
  (params (Points :type Integer))
  (bind _output_get (Variables|Default|SetPoints (+ Points (Variables|Default|GetPoints))))
  (if (== _output_get (Variables|Default|GetTotalPoints))
    (Variables|Default|SetWin true)
    (CallFunction|ResetTimer)))

(fn ConstructionScript)