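; Inventory component that tracks how many of each ingredient is held, apparently for a cauldron system.
; Counts live in an enum-keyed map; AddToInventory adds an amount to the stored value and prints the new total.
; CheckInventoryCount returns the count for a given type after converting it to the ingredient enum.
; Debug output prints a greeting on BeginPlay and every map entry on each Tick.
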(event EventBeginPlay
  (Development|PrintString "Hello from BPC_Inventory"))

(event EventTick
  (params (DeltaSeconds :type Float%20%28single-precision%29))
  (bind (_keypin _valuepin) (Utilities|Map|ForEachLoop(Map) (Variables|Default|GetEnumInventory))
    (:then
      (Development|PrintText (Utilities|Text|FormatText "{Key}:{Value}" (Utilities|String|EnumtoString _keypin) _valuepin) true true "(R=0.000000,G=0.660000,B=1.000000,A=1.000000)" 1.0))))

(fn CheckInventoryCount
  (params (Type :type Byte :default 0))
  (return (.Value (Utilities|Map|Find (Variables|Default|GetEnumInventory) (Utilities|Enum|ByteToEnumE_Ingredients Type)))))

(fn AddtoInventory
  (params (Ingredient :type E_Ingredients%20Enum :default "NewEnumerator0") (Amount :type Integer))
  (bind _enuminventory (Variables|Default|GetEnumInventory))
  (Utilities|Map|Add _enuminventory Ingredient (+ (.Value (Utilities|Map|Find _enuminventory Ingredient)) Amount))
  (Development|PrintText (Utilities|Text|FormatText "We now have {amount} {ingredient}" (.Value (Utilities|Map|Find _enuminventory Ingredient)) (Utilities|String|EnumtoString Ingredient))))