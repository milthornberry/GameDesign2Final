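; BP_TrialPoint is a time trial point that an overlapping actor collects while its particle effect is active.
; The particle system doubles as the armed state and is switched off on BeginPlay and TimeTrialReset, with no activation in this Blueprint.
; A Box overlap while it is active deactivates the effect and sends TimeTrialCountMessage with a count of one to the overlapping actor.
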(event OnComponentBeginOverlap(Box)
  (params (OverlappedComponent :type Primitive%20Component%20Object%20Reference) (OtherActor :type Actor%20Object%20Reference) (OtherComp :type Primitive%20Component%20Object%20Reference) (OtherBodyIndex :type Integer) (bFromSweep :type Boolean) (SweepResult :type Hit%20Result%20Structure%20%28by%20ref%29))
  (if (Components|Activation|IsActive (Variables|Default|GetParticleSystem))
    (Components|Activation|Deactivate (Variables|Default|GetParticleSystem))
    (Class|BPITimeTrial|TimeTrialCount(Message) OtherActor 1)))

(event EventBeginPlay
  (Components|Activation|Deactivate (Variables|Default|GetParticleSystem)))

(event EventTimeTrialReset
  (Components|Activation|Deactivate (Variables|Default|GetParticleSystem)))

(fn ConstructionScript)