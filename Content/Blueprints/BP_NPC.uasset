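; NPC that shows voiced dialogue from DT_NPCDialogue when BP_ThirdPersonCharacter enters its sphere.
; Overlap registers the NPC on the player and shows W_Dialogue; leaving or passing the last row hides it and resets to StartingLineIndex.
; NextLine steps through rows by index, setting text and playing audio, but stalls on a "<-------->" separator row without ending the dialogue.
; Speaker-based text angle and justification currently resolve identically for both options.
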(event OnComponentBeginOverlap(Sphere)
  (params (OverlappedComponent :type Primitive%20Component%20Object%20Reference) (OtherActor :type Actor%20Object%20Reference) (OtherComp :type Primitive%20Component%20Object%20Reference) (OtherBodyIndex :type Integer) (bFromSweep :type Boolean) (SweepResult :type Hit%20Result%20Structure%20%28by%20ref%29))
  (bind _asbp_third_person_character (Utilities|Casting|CastToBP_ThirdPersonCharacter OtherActor))
  (bind _output_get (Variables|Default|SetPlayer _asbp_third_person_character))
  (Variables|/Game/Blueprints/BP_ThirdPersonCharacter.BP_ThirdPersonCharacter_C|SetNPC _output_get self)
  (UserInterface|Viewport|AddtoViewport (Variables|Default|GetW_Dialogue) 0)
  (CallFunction|NextLine))

(event OnComponentEndOverlap(Sphere)
  (params (OverlappedComponent :type Primitive%20Component%20Object%20Reference) (OtherActor :type Actor%20Object%20Reference) (OtherComp :type Primitive%20Component%20Object%20Reference) (OtherBodyIndex :type Integer))
  (Utilities|Casting|CastToBP_ThirdPersonCharacter OtherActor)
  (CallFunction|EndDialogue))

(event Custom|Next%20Line
  (bind _audio (Variables|Default|GetAudio))
  (bind _w_dialogue (Variables|Default|GetW_Dialogue))
  (bind _textblock_0 (Variables|/Game/Widgets/W_Dialogue.W_Dialogue_C|GetTextBlock_0 _w_dialogue))
  (bind _outrownames (DataTable|GetDataTableRowNames 0))
  (if (> (Variables|Default|GetNext%20Line%20Index) (Utilities|Array|LastIndex _outrownames)) ; Are we at the end of the dialogue?
    (CallFunction|EndDialogue)
    (else
      (bind _returnvalue (Utilities|GetDataTableRow "/Game/Blueprints/DT_NPCDialogue.DT_NPCDialogue" (Utilities|Array|Get(acopy) _outrownames (Variables|Default|GetNext%20Line%20Index)))
        (:then
          (if (not (Utilities|Enum|Equal(Enum) (Utilities|String|ToString(Text) (.dialogueline _returnvalue)) "<-------->"))
            (Rendering|Components|TextRender|SetText (Variables|/Game/Widgets/W_Dialogue.W_Dialogue_C|GetTextBlock_0 (Variables|Default|GetW_Dialogue)) (Utilities|Text|ToText(String) (Utilities|String|ToString(Text) (.dialogueline _returnvalue))))
            (Math|Integer|IncrementInt (Variables|Default|GetNext%20Line%20Index)
              (:%20%20
                (Audio|Components|Audio|SetSound _audio (.voicedline _returnvalue))
                (Audio|Components|Audio|Play _audio 0.0)
                (Class|Widget|SetRenderTransformAngle _textblock_0 (Utilities|Select :Index (.speaker _returnvalue) :Option%200 0.0 :Option%201 0.0))
                (Variables|/Script/UMG.TextLayoutWidget|SetJustification _textblock_0 (Utilities|Select :Index (.speaker _returnvalue) :Option%200 "Left" :Option%201 "Left"))))))))))

(event Custom|End%20dialogue
  (Variables|/Game/Blueprints/BP_ThirdPersonCharacter.BP_ThirdPersonCharacter_C|SetNPC (Variables|Default|GetPlayer) 0)
  (Variables|Default|SetPlayer 0) ; Set player to null
  (Widget|RemovefromParent (Variables|Default|GetW_Dialogue)) ; Hides the dialogue
  (Variables|Default|SetNext%20Line%20Index (Variables|Default|GetStarting%20Line%20Index)))

(event EventBeginPlay
  (bind _returnvalue (UserInterface|CreateWidget "/Game/Widgets/W_Dialogue.W_Dialogue_C")) ; Gets the widget ready to show
  (Variables|Default|SetW_Dialogue _returnvalue)
  (Variables|Default|SetNext%20Line%20Index (Variables|Default|GetStarting%20Line%20Index)))

(fn ConstructionScript)